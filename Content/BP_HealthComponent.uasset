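; BP_HealthComponent holds a normalized health value and feeds it to the HUD through an MVVM viewmodel.
; On BeginPlay it creates a UVM_Health, registers it in the global viewmodel collection and hands it to the health widget on BP_ThirdPersonHUD.
; ChangeHealth steps health within 0–1, reversing direction at either end, like a test driver.
; It derives a three-tier status, pushes both values to the viewmodel and prints health.
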(event `self.ReceiveBeginPlay`
  (bind _returnvalue (`|GenericCreateObject` "/Game/UI/UVM_Health.UVM_Health_C"))
  (bind _output_get (set `self.UVM_Health` _returnvalue))
  (`MVVMViewModelCollectionObject.AddViewModelInstance` (`MVVMGameSubsystem.GetViewModelCollection` (subsystem `MVVMGameSubsystem`)) (make `MVVMViewModelContext` "/Game/UI/UVM_Health.UVM_Health_C" "HealthViewModel") _output_get)
  (bind _asbp_third_person_hud (cast `/Game/ThirdPerson/Blueprints/BP_ThirdPersonHUD` (`PlayerController.GetHUD` (`GameplayStatics.GetPlayerController` 0))))
  (`/Game/UI/Widgets/WBP_Health.SetUVM_Health` (`/Game/UI/Widgets/WBP_HUD.WBP_Health` (`/Game/ThirdPerson/Blueprints/BP_ThirdPersonHUD.WBP_HUD` _asbp_third_person_hud)) (`self.UVM_Health`)))

(fn `changeHealth`
  (bind _health (`self.Health`))
  (bind _output_get (set `self.Health` (`KismetMathLibrary.FClamp` (+ (`self.Health`) (`self.HealthChangeAmount`)))))
  (set `/Game/UI/UVM_Health.HealthPercent` _output_get (`self.UVM_Health`))
  (if (or (`KismetMathLibrary.NearlyEqual_FloatFloat` (`self.Health`) 0.0 0.01) (`KismetMathLibrary.NearlyEqual_FloatFloat` (`self.Health`) 1.0 0.01))
    (set `self.HealthChangeAmount` (* (`self.HealthChangeAmount`) -1.0)))
  (if (< _health 0.01)
    (set `self.HealthStatus` "NewEnumerator2")
    (elif (< (`self.Health`) 0.25)
      (set `self.HealthStatus` "NewEnumerator1")
      (else
        (set `self.HealthStatus` "NewEnumerator0"))))
  (set `/Game/UI/UVM_Health.HealthStatus` (`self.HealthStatus`) (`self.UVM_Health`))
  (`KismetSystemLibrary.PrintString` (`KismetStringLibrary.Conv_DoubleToString` _health)))